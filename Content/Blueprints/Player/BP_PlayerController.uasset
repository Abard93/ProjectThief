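; Player controller that implements click-to-move for the controlled pawn.
; The SetDestination input opens a Gate on press and closes it on release, with the gate's exit running a complex Camera-channel trace under the cursor.
; MoveToHitLocation sends the pawn to the hit point with SimpleMoveToLocation, skipping points closer to the pawn than MinClickDistance.
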(event `self.ReceiveTick`
  (params (DeltaSeconds :type "Float (single-precision)"))
  ;[1 1 1] Click and go there
)

(event `InputAction|SetDestination`
  (params (Key :type "Key Structure"))
  ;[1 1 1] Click and go there
  (:`Pressed`
    (`/Engine/EditorBlueprintResources/StandardMacros.Gate` true :!via `Open` :!label _label ; While key is pressed...
      (:`Exit`
        (`self.MoveToHitLocation` (`self.GetHitResultUnderCursorByChannel` "TraceTypeQuery2")))))
  (:`Released`
    (goto _label :!via `Close`)))

(fn `MoveToHitLocation`
  (params (InputHit :type "HitResult Structure"))
  (bind (_bblockinghit _binitialoverlap _time _distance _location) (`GameplayStatics.BreakHitResult` InputHit))
  (if (>= (`KismetMathLibrary.VSize` (- (`self.K2_GetActorLocation` (`self.K2_GetPawn`)) _location)) (`self.MinClickDistance`))
    (`AIBlueprintHelperLibrary.SimpleMoveToLocation` self _location)))

(fn `UserConstructionScript`)